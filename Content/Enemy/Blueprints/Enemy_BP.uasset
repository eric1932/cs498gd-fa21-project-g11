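; Enemy character Blueprint that chases the first-person player and attacks at close range.
; Tick issues AI MoveTo toward the player while alive; reaching attack range holds an Attacking flag for a fixed delay.
; AttackPlayer, not called within this Blueprint, damages the player if within hit distance.
; TakeDamage reduces health, then at zero flags death, disables mesh collision and stops movement.
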(event `self.ReceiveBeginPlay`
  (bind _asfirst_person_character (cast `/Game/FirstPersonBP/Blueprints/FirstPersonCharacter` (`GameplayStatics.GetPlayerCharacter` 0)))
  (set `self.Player` _asfirst_person_character))

(event `self.ReceiveActorBeginOverlap`
  (params (OtherActor :type "Actor Object Reference")))

(event `self.ReceiveTick`
  (params (DeltaSeconds :type "Float (single-precision)"))
  (if (not (`self.Dead`))
    (`|AIMoveTo` self (0.0 0.0 0.0) (`self.Player`) (`self.AttackStartDistance`) true
      (:`OnSuccess`
        (if (not (`self.Attacking`))
          (set `self.Attacking` true)
          (`KismetSystemLibrary.Delay` 2.6)
          (set `self.Attacking` false))))))

(fn `AttackPlayer`
  (if (<= (`KismetMathLibrary.Vector_Distance` (`self.K2_GetActorLocation`) (`self.K2_GetActorLocation` (`self.Player`))) (`self.AttackHitDistance`))
    (`/Game/FirstPersonBP/Blueprints/FirstPersonCharacter.TakeDamage` (`self.Player`))))

(fn `TakeDamage`
  (params (DamageToTake :type Integer))
  (bind _output_get (set `self.Health` (- (`self.Health`) DamageToTake)))
  (if (<= _output_get 0)
    (set `self.Dead` true)
    (`PrimitiveComponent.SetCollisionEnabled` (`self.Mesh`) "NoCollision")
    (`MovementComponent.StopMovementImmediately` (`self.CharacterMovement`))))

(fn `UserConstructionScript`)